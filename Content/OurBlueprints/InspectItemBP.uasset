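; Inspectable item actor that the player can pull up to examine, doubling as the flashlight pickup.
; Inspect enables input and runs a timeline moving the actor to the player's InspectPoint with collision off, where mouse axes rotate the mesh.
; Pressing E ends inspection: normal items reverse back, reset rotation and restore collision.
; Items flagged IsFlashlight instead shrink away, set HasFlashlight on the player and destroy themselves.
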(event Custom|InspectAnim
  (params (PlayerRef :type BP%20First%20Person%20Character%20Object%20Reference))
  (Utilities|FlowControl|Sequence
    (:then_0
      (Input|EnableInput (Game|GetPlayerController 0)))
    (:then_1
      (bind _newtrack_0 (Timeline|Timeline Play)
        (:Update
          (Transformation|SetActorLocation (Math|Vector|Lerp(Vector) (Variables|Default|GetActorInspectAnimStartLoc) (Transformation|GetWorldLocation (Variables|/Game/FirstPerson/Blueprints/BP_FirstPersonCharacter.BP_FirstPersonCharacter_C|GetInspectPoint PlayerRef)) _newtrack_0) false false)
          (Collision|SetCollisionEnabled (Variables|Default|GetStaticMesh) "NoCollision"))))))

(event EventBeginPlay
  (Variables|Default|SetActorInspectAnimStartLoc (Transformation|GetActorLocation)))

(event Input|MouseEvents|MouseX
  (params (AxisValue :type Float%20%28single-precision%29))
  (Transformation|AddLocalRotation (Variables|Default|GetStaticMesh) (Math|Rotator|MakeRotator 0.0 0.0 AxisValue) false false))

(event Input|MouseEvents|MouseY
  (params (AxisValue :type Float%20%28single-precision%29))
  (Transformation|AddLocalRotation (Variables|Default|GetStaticMesh) (Math|Rotator|MakeRotator AxisValue 0.0 0.0) false false))

(event Input|KeyboardEvents|E
  (params (Key :type Key%20Structure :default "None"))
  (bind _staticmesh (Variables|Default|GetStaticMesh))
  (bind _staticmesh_2 (Variables|Default|GetStaticMesh))
  (:Pressed
    (Utilities|FlowControl|Sequence
      (:then_0
        (if (not (Variables|Default|GetisFlashlight))
          (bind _newtrack_0 (Timeline|Timeline Reverse)
            (:Update
              (Transformation|SetActorLocation (Math|Vector|Lerp(Vector) (Variables|Default|GetActorInspectAnimStartLoc) (Transformation|GetWorldLocation (Variables|/Game/FirstPerson/Blueprints/BP_FirstPersonCharacter.BP_FirstPersonCharacter_C|GetInspectPoint (stale Custom|InspectAnim PlayerRef))) _newtrack_0) false false)
              (Collision|SetCollisionEnabled (Variables|Default|GetStaticMesh) "NoCollision")))))
      (:then_1
        (Input|DisableInput (Game|GetPlayerController 0))
        (Default|StopInspectingItem (stale Custom|InspectAnim PlayerRef))
        (if (not (Variables|Default|GetisFlashlight))
          (bind _newtrack_0_2 (Timeline|Timeline_0 PlayFromStart)
            (:Update
              (Transformation|SetRelativeRotation _staticmesh_2 (Math|Rotator|Lerp(Rotator) (Variables|/Script/Engine.SceneComponent|GetRelativeRotation _staticmesh_2) (Math|Rotator|MakeRotator 0.0 0.0 0.0) _newtrack_0_2) false false)
              (Collision|SetCollisionEnabled (Variables|Default|GetStaticMesh) "QueryAndPhysics")))
          (else
            (bind _newtrack_0_3 (Timeline|Timeline_1 PlayFromStart)
              (:Update
                (Transformation|SetWorldScale3D _staticmesh (Math|Vector|Lerp(Vector) (Transformation|GetWorldScale _staticmesh) "0, 0, 0" _newtrack_0_3)))
              (:Finished
                (Variables|/Game/FirstPerson/Blueprints/BP_FirstPersonCharacter.BP_FirstPersonCharacter_C|SethasFlashlight (stale Custom|InspectAnim PlayerRef) true)
                (Utilities|FlowControl|Delay 0.2)
                (Actor|DestroyActor)))))))))

(fn ConstructionScript)

(fn Inspect
  (params (PlayerRef :type BP%20First%20Person%20Character%20Object%20Reference))
  (CallFunction|InspectAnim PlayerRef))