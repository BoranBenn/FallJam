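; BP_Note1 is a collectible note actor that the player picks up through an Interact event.
; On BeginPlay it creates its own W_Notes widget and adds it to the viewport.
; Interact plays a paper sound at the Plane component, copies its IsSolAlt (bottom-left) variable into the widget's IsSolAltTaken, then destroys the actor after a short delay.
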(event EventBeginPlay
  (bind _returnvalue (UserInterface|CreateWidget "/Game/OurBlueprints/W_Notes.W_Notes_C"))
  (bind _output_get (Variables|Default|SetWnotes _returnvalue))
  (UserInterface|Viewport|AddtoViewport _output_get 0))

(event Collision|EventActorBeginOverlap
  (params (OtherActor :type Actor%20Object%20Reference)))

(event EventTick
  (params (DeltaSeconds :type Float%20%28single-precision%29)))

(event EventInteract
  (Audio|PlaySoundatLocation "/Game/OurBlueprints/Sounds/kagit_2.kagit_2" (Transformation|GetWorldLocation (Variables|Default|GetPlane)) "0, 0, 0" 1.0 1.0 0.0 0 0 0 0)
  (Variables|/Game/OurBlueprints/W_Notes.W_Notes_C|SetIsSolAltTaken (Variables|Default|GetWnotes) (Variables|Default|GetIsSolAlt))
  (Utilities|FlowControl|Delay 0.2)
  (Actor|DestroyActor))

(fn ConstructionScript)