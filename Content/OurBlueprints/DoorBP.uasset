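; DoorBP is a sliding double-door actor with a trigger that brings up a password prompt.
; On BeginPlay, a Timeline slides Cube1 and Cube in opposite directions along world X from the actor's location by Amount.
; Any Box overlap creates a Password_W widget, switches input to UI only and shows the cursor.
; The door motion is not gated by the password in this graph.
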(event OnComponentBeginOverlap(Box)
  (params (OverlappedComponent :type Primitive%20Component%20Object%20Reference) (OtherActor :type Actor%20Object%20Reference) (OtherComp :type Primitive%20Component%20Object%20Reference) (OtherBodyIndex :type Integer) (bFromSweep :type Boolean) (SweepResult :type Hit%20Result%20Structure%20%28by%20ref%29))
  (bind _returnvalue (Game|GetPlayerController 0))
  (bind _returnvalue_2 (UserInterface|CreateWidget "/Game/OurBlueprints/Password_W.Password_W_C" _returnvalue))
  (UserInterface|Viewport|AddtoPlayerScreen _returnvalue_2)
  (Input|SetInputModeUIOnly _returnvalue _returnvalue_2 "DoNotLock" true)
  (Variables|/Script/Engine.PlayerController|SetbShowMouseCursor _returnvalue true))

(event EventBeginPlay
  (bind _returnvalue (Transformation|GetActorLocation))
  (bind _newtrack_0 (Timeline|Timeline Play)
    (:Update
      (Transformation|SetWorldLocation (Variables|Default|GetCube1) (Math|Vector|Lerp(Vector) _returnvalue (+ _returnvalue (Math|Vector|MakeVector (Variables|Default|GetAmount) 0.0 0.0)) _newtrack_0) false false)
      (Transformation|SetWorldLocation (Variables|Default|GetCube) (Math|Vector|Lerp(Vector) _returnvalue (+ _returnvalue (Math|Vector|MakeVector (* (Variables|Default|GetAmount) -1.0) 0.0 0.0)) _newtrack_0) false false))))

(fn ConstructionScript)