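; BP_RandomObject is an interactable actor whose Cube the first-person player can pick up and drop.
; BeginPlay caches the player's BP_FirstPersonCharacter, and each Interact call toggles the IsTaken flag.
; Picking up attaches the Cube to the character's capsule at its current world location, and dropping detaches it, keeping its world transform.
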(event EventBeginPlay
  (bind _asbp_first_person_character (Utilities|Casting|CastToBP_FirstPersonCharacter (Game|GetPlayerCharacter 0)))
  (Variables|Default|SetAs%20BP%20First%20Person%20Character _asbp_first_person_character))

(event Collision|EventActorBeginOverlap
  (params (OtherActor :type Actor%20Object%20Reference)))

(event EventInteract
  (bind _cube (Variables|Default|GetCube))
  (if (Variables|Default|GetIsTaken)
    (if (Variables|Default|GetIsTaken)
      (Transformation|DetachFromComponent _cube "KeepWorld" "KeepWorld" "KeepWorld" false)
      (Variables|Default|SetIsTaken false))
    (else
      (bind _output_get (Variables|Default|SetIsTaken true))
      (if _output_get
        (Transformation|AttachComponentToComponent _cube (Variables|/Script/Engine.Character|GetCapsuleComponent (Variables|Default|GetAs%20BP%20First%20Person%20Character)) "None" "KeepWorld" "KeepRelative" "KeepRelative" true)))))

(fn ConstructionScript)