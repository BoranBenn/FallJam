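; Interactable spotlight actor that the player takes control of and aims using the movement axes.
; Interact or E toggles control, swapping input with BP_FirstPersonCharacter and moving its camera to CamPoint, then restoring it on exit.
; MoveRight and MoveForward set RotatingMovement's yaw and pitch rates from Speed, with leftover debug prints.
; Tick, enabled on entering control and disabled on exit, zeroes roll so the camera stays level.
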(event EventTick
  (params (DeltaSeconds :type Float%20%28single-precision%29))
  (bind _returnvalue (Transformation|GetActorRotation))
  ;[0.15 0.15 0.15 0.5] kamera yan yatmasın diye X'i sabitliyorum. belki daha iyi bi yolu vardır idk
  (Transformation|SetActorRotation (Math|Rotator|MakeRotator 0.0 (.pitch _returnvalue) (.yaw _returnvalue))))

(event EventInteract
  (bind _returnvalue (Game|GetPlayerController 0))
  (bind _returnvalue_2 (Game|GetPlayerController 0))
  (bind _campoint (Variables|Default|GetCamPoint))
  (bind _output_get (Variables|Default|SetinInteraction (not (Variables|Default|GetinInteraction))))
  (if _output_get
    (Input|EnableInput _returnvalue)
    (bind _asbp_first_person_character (Utilities|Casting|CastToBP_FirstPersonCharacter (Game|Player|GetPlayerPawn 0)))
    (Utilities|FlowControl|Sequence
      (:then_0
        (Components|Movement|StopMovementImmediately (Variables|/Script/Engine.Character|GetCharacterMovement _asbp_first_person_character))
        (Input|DisableInput _asbp_first_person_character _returnvalue_2)
        (Components|Activation|SetActive (Variables|Default|GetRotatingMovement) true true))
      (:then_1
        (Variables|Default|SetcamStartTrans (Transformation|GetWorldTransform (Variables|/Game/FirstPerson/Blueprints/BP_FirstPersonCharacter.BP_FirstPersonCharacter_C|GetFirstPersonCamera _asbp_first_person_character)))
        (Variables|/Script/Engine.CameraComponent|SetbUsePawnControlRotation (Variables|/Game/FirstPerson/Blueprints/BP_FirstPersonCharacter.BP_FirstPersonCharacter_C|GetFirstPersonCamera _asbp_first_person_character) false)
        (Transformation|SetWorldLocationAndRotation (Variables|/Game/FirstPerson/Blueprints/BP_FirstPersonCharacter.BP_FirstPersonCharacter_C|GetFirstPersonCamera _asbp_first_person_character) (Transformation|GetWorldLocation _campoint) (Transformation|GetWorldRotation _campoint) false false)
        (Transformation|DetachFromComponent (Variables|/Game/FirstPerson/Blueprints/BP_FirstPersonCharacter.BP_FirstPersonCharacter_C|GetFirstPersonCamera _asbp_first_person_character) "KeepWorld" "KeepWorld" "KeepWorld" true)
        (Utilities|FlowControl|Delay 0.2)
        (Transformation|AttachComponentToComponent (Variables|/Game/FirstPerson/Blueprints/BP_FirstPersonCharacter.BP_FirstPersonCharacter_C|GetFirstPersonCamera _asbp_first_person_character) (Variables|Default|GetCamPoint) "None" "KeepWorld" "KeepWorld" "KeepWorld" true)
        (Actor|Tick|SetActorTickEnabled true)))
    (else
      (Input|DisableInput _returnvalue)
      (bind _asbp_first_person_character_2 (Utilities|Casting|CastToBP_FirstPersonCharacter (Game|Player|GetPlayerPawn 0)))
      (Input|EnableInput _asbp_first_person_character_2 _returnvalue_2)
      (Variables|/Script/Engine.CameraComponent|SetbUsePawnControlRotation (Variables|/Game/FirstPerson/Blueprints/BP_FirstPersonCharacter.BP_FirstPersonCharacter_C|GetFirstPersonCamera _asbp_first_person_character) true)
      (Transformation|AttachComponentToComponent (Variables|/Game/FirstPerson/Blueprints/BP_FirstPersonCharacter.BP_FirstPersonCharacter_C|GetFirstPersonCamera _asbp_first_person_character) (Variables|/Game/FirstPerson/Blueprints/BP_FirstPersonCharacter.BP_FirstPersonCharacter_C|GetFirstPersonMesh _asbp_first_person_character) "None" "KeepWorld" "KeepWorld" "KeepWorld" true)
      (Transformation|SetWorldTransform (Variables|/Game/FirstPerson/Blueprints/BP_FirstPersonCharacter.BP_FirstPersonCharacter_C|GetFirstPersonCamera _asbp_first_person_character) (Variables|Default|GetcamStartTrans) false false)
      (Actor|Tick|SetActorTickEnabled false)
      (Components|Activation|SetActive (Variables|Default|GetRotatingMovement) false true))))

(event Input|AxisEvents|InputAxisMoveForward
  (params (AxisValue :type Float%20%28single-precision%29))
  (bind _rotatingmovement (Variables|Default|GetRotatingMovement))
  (bind _rotatingmovement_2 (Variables|Default|GetRotatingMovement))
  (bind _rotatingmovement_3 (Variables|Default|GetRotatingMovement))
  (if (== AxisValue 1.0)
    (Variables|/Script/Engine.RotatingMovementComponent|SetRotationRate _rotatingmovement (Math|Rotator|MakeRotator 0.0 (Variables|Default|Getspeed) (.yaw (Variables|/Script/Engine.RotatingMovementComponent|GetRotationRate _rotatingmovement))))
    (Development|PrintString "1")
    (elif (== AxisValue -1.0)
      (Variables|/Script/Engine.RotatingMovementComponent|SetRotationRate _rotatingmovement_3 (Math|Rotator|MakeRotator 0.0 (* (Variables|Default|Getspeed) -1.0) (.yaw (Variables|/Script/Engine.RotatingMovementComponent|GetRotationRate _rotatingmovement_3))))
      (Development|PrintString "2")
      (elif (== AxisValue 0.0)
        (Variables|/Script/Engine.RotatingMovementComponent|SetRotationRate _rotatingmovement_2 (Math|Rotator|MakeRotator 0.0 0.0 (.yaw (Variables|/Script/Engine.RotatingMovementComponent|GetRotationRate _rotatingmovement_2))))
        (Development|PrintString "3")
        (else
          (Development|PrintString "Hello"))))))

(event Input|AxisEvents|InputAxisMoveRight
  (params (AxisValue :type Float%20%28single-precision%29))
  (bind _returnvalue (== AxisValue 0.0))
  (bind _rotatingmovement (Variables|Default|GetRotatingMovement))
  (bind _rotatingmovement_2 (Variables|Default|GetRotatingMovement))
  (bind _rotatingmovement_3 (Variables|Default|GetRotatingMovement))
  (if (== AxisValue 1.0)
    (Variables|/Script/Engine.RotatingMovementComponent|SetRotationRate _rotatingmovement_2 (Math|Rotator|MakeRotator 0.0 (.pitch (Variables|/Script/Engine.RotatingMovementComponent|GetRotationRate _rotatingmovement_2)) (Variables|Default|Getspeed)))
    (elif (== AxisValue -1.0)
      (Variables|/Script/Engine.RotatingMovementComponent|SetRotationRate _rotatingmovement_3 (Math|Rotator|MakeRotator 0.0 (.pitch (Variables|/Script/Engine.RotatingMovementComponent|GetRotationRate _rotatingmovement_3)) (* (Variables|Default|Getspeed) -1.0)))
      (elif _returnvalue
        (Variables|/Script/Engine.RotatingMovementComponent|SetRotationRate _rotatingmovement (Math|Rotator|MakeRotator 0.0 (.pitch (Variables|/Script/Engine.RotatingMovementComponent|GetRotationRate _rotatingmovement)) 0.0))
        (elif (and _returnvalue (== (stale Input|AxisEvents|InputAxisMoveForward AxisValue) 0.0))
          (Variables|/Script/Engine.RotatingMovementComponent|SetRotationRate (Variables|Default|GetRotatingMovement) "0, 0, 0"))))))

(event Input|KeyboardEvents|E
  (params (Key :type Key%20Structure :default "None"))
  (bind _returnvalue (Game|GetPlayerController 0))
  (bind _returnvalue_2 (Game|GetPlayerController 0))
  (bind _campoint (Variables|Default|GetCamPoint))
  (:Pressed
    (bind _output_get (Variables|Default|SetinInteraction (not (Variables|Default|GetinInteraction))))
    (if _output_get
      (Input|EnableInput _returnvalue)
      (bind _asbp_first_person_character (Utilities|Casting|CastToBP_FirstPersonCharacter (Game|Player|GetPlayerPawn 0)))
      (Utilities|FlowControl|Sequence
        (:then_0
          (Components|Movement|StopMovementImmediately (Variables|/Script/Engine.Character|GetCharacterMovement _asbp_first_person_character))
          (Input|DisableInput _asbp_first_person_character _returnvalue_2)
          (Components|Activation|SetActive (Variables|Default|GetRotatingMovement) true true))
        (:then_1
          (Variables|Default|SetcamStartTrans (Transformation|GetWorldTransform (Variables|/Game/FirstPerson/Blueprints/BP_FirstPersonCharacter.BP_FirstPersonCharacter_C|GetFirstPersonCamera _asbp_first_person_character)))
          (Variables|/Script/Engine.CameraComponent|SetbUsePawnControlRotation (Variables|/Game/FirstPerson/Blueprints/BP_FirstPersonCharacter.BP_FirstPersonCharacter_C|GetFirstPersonCamera _asbp_first_person_character) false)
          (Transformation|SetWorldLocationAndRotation (Variables|/Game/FirstPerson/Blueprints/BP_FirstPersonCharacter.BP_FirstPersonCharacter_C|GetFirstPersonCamera _asbp_first_person_character) (Transformation|GetWorldLocation _campoint) (Transformation|GetWorldRotation _campoint) false false)
          (Transformation|DetachFromComponent (Variables|/Game/FirstPerson/Blueprints/BP_FirstPersonCharacter.BP_FirstPersonCharacter_C|GetFirstPersonCamera _asbp_first_person_character) "KeepWorld" "KeepWorld" "KeepWorld" true)
          (Utilities|FlowControl|Delay 0.2)
          (Transformation|AttachComponentToComponent (Variables|/Game/FirstPerson/Blueprints/BP_FirstPersonCharacter.BP_FirstPersonCharacter_C|GetFirstPersonCamera _asbp_first_person_character) (Variables|Default|GetCamPoint) "None" "KeepWorld" "KeepWorld" "KeepWorld" true)
          (Actor|Tick|SetActorTickEnabled true)))
      (else
        (Input|DisableInput _returnvalue)
        (bind _asbp_first_person_character_2 (Utilities|Casting|CastToBP_FirstPersonCharacter (Game|Player|GetPlayerPawn 0)))
        (Input|EnableInput _asbp_first_person_character_2 _returnvalue_2)
        (Variables|/Script/Engine.CameraComponent|SetbUsePawnControlRotation (Variables|/Game/FirstPerson/Blueprints/BP_FirstPersonCharacter.BP_FirstPersonCharacter_C|GetFirstPersonCamera _asbp_first_person_character) true)
        (Transformation|AttachComponentToComponent (Variables|/Game/FirstPerson/Blueprints/BP_FirstPersonCharacter.BP_FirstPersonCharacter_C|GetFirstPersonCamera _asbp_first_person_character) (Variables|/Game/FirstPerson/Blueprints/BP_FirstPersonCharacter.BP_FirstPersonCharacter_C|GetFirstPersonMesh _asbp_first_person_character) "None" "KeepWorld" "KeepWorld" "KeepWorld" true)
        (Transformation|SetWorldTransform (Variables|/Game/FirstPerson/Blueprints/BP_FirstPersonCharacter.BP_FirstPersonCharacter_C|GetFirstPersonCamera _asbp_first_person_character) (Variables|Default|GetcamStartTrans) false false)
        (Actor|Tick|SetActorTickEnabled false)
        (Components|Activation|SetActive (Variables|Default|GetRotatingMovement) false true)))))

(fn ConstructionScript)