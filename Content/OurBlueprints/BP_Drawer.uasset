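; BP_Drawer is an interactable drawer that slides open and closed and can hold a spawned note.
; On BeginPlay, if SpawnNote is set, it spawns a BP_Note2 and attaches it to the SolDrawer component.
; Interact alternates through a FlipFlop, setting IsOpen and playing or reversing a Timeline that drives the drawer's relative Y position.
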(event EventBeginPlay
  (if (Variables|Default|GetspawnNote)
    (bind _returnvalue (Game|SpawnActorfromClass "/Game/OurBlueprints/BP_Note2.BP_Note2_C" (Variables|Default|GetSpawn%20Transform) "Undefined" "MultiplyWithRoot" 0 0))
    (bind _output_get (Variables|Default|SetNewVar _returnvalue))
    (Transformation|AttachComponentToComponent _output_get (Variables|Default|GetSolDrawer) "None" "KeepRelative" "KeepRelative" "KeepRelative" true)))

(event Collision|EventActorBeginOverlap
  (params (OtherActor :type Actor%20Object%20Reference)))

(event EventTick
  (params (DeltaSeconds :type Float%20%28single-precision%29)))

(event EventInteract
  (bind _soldrawer (Variables|Default|GetSolDrawer))
  (bind _relativelocation (Variables|/Script/Engine.SceneComponent|GetRelativeLocation _soldrawer))
  (Utilities|FlowControl|FlipFlop
    (:A
      (bind _output_get (Variables|Default|SetIsOpen true))
      (if _output_get
        (bind _newtrack_0 (Timeline|Timeline Play)
          (:Update
            (Transformation|SetRelativeLocation _soldrawer (Math|Vector|MakeVector (.x _relativelocation) _newtrack_0 (.z _relativelocation)) false false)))))
    (:B
      (bind _output_get_2 (Variables|Default|SetIsOpen false))
      (if (not _output_get_2)
        (Timeline|Timeline Reverse)))))

(fn ConstructionScript)